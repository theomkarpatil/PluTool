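; Builder-mode visualiser that shows a ghost preview of the selected block in front of the player while the PluTool UI is in the viewport.
; On Tick, a BlockIndex change spawns that DT_BBList row's block, tinted blue or red by its prerequisite check against BlocksInScene.
; The preview receives a grid-snapped camera-forward position each frame.
; Placed blocks get BaseMaterial and join BlocksInScene; leaving builder mode destroys the preview.
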(event EventBeginPlay)

(event Collision|EventActorBeginOverlap
  (params (OtherActor :type Actor%20Object%20Reference)))

(event EventTick
  (params (DeltaSeconds :type Float%20%28single-precision%29))
  ;[0.08854 0.08854 0.08854] Making sure we're in Builder mode
  (bind _foundwidgets (Widget|GetAllWidgetsOfClass "/Game/PluToolAssets/Blueprints/UI/BP_PluToolUI.BP_PluToolUI_C" true))
  (if (> (Utilities|Array|Length _foundwidgets) 0)
    (if (UserInterface|Viewport|IsinViewport (Utilities|Array|Get(acopy) _foundwidgets))
      (bind _asbp_first_person_character (Utilities|Casting|CastToBP_FirstPersonCharacter (Game|GetPlayerCharacter 0)))
      (if (== (Variables|/Game/FirstPerson/Blueprints/BP_FirstPersonCharacter.BP_FirstPersonCharacter_C|GetBlockIndex _asbp_first_person_character) (Variables|Default|GetprevIndex))
        ;[0.05208 0.05208 0.05208] Setting values for the current block so that it follows player view
        (if (Utilities|IsValid (Variables|Default|GetmVisibleBlock))
          (Utilities|FlowControl|Sequence
            (:then_0
              (if (Variables|/Script/PluTool.BuilderBlock|GetmMeetsPrerequisites (Variables|Default|GetmVisibleBlock))
                (Rendering|Material|SetMaterial (Variables|/Script/PluTool.BuilderBlock|GetmMesh (Variables|Default|GetmVisibleBlock)) 0 "/Game/PluToolAssets/Assets/Materials/M_BlueTrans.M_BlueTrans")
                (else
                  (Rendering|Material|SetMaterial (Variables|/Script/PluTool.BuilderBlock|GetmMesh (Variables|Default|GetmVisibleBlock)) 0 "/Game/PluToolAssets/Assets/Materials/M_RedTrans.M_RedTrans"))))
            (:then_1
              (Variables|/Script/PluTool.BuilderBlock|SetmNewBlockPosition (Variables|Default|GetmVisibleBlock) (+ (Class|KismetMathLibrary|VectorSnappedtoGrid (+ (Transformation|GetActorLocation _asbp_first_person_character) (* (Math|Vector|GetForwardVector (Variables|/Game/FirstPerson/Blueprints/BP_FirstPersonCharacter.BP_FirstPersonCharacter_C|GetFirstPersonCamera _asbp_first_person_character)) "750.000000,750.000000,750.000000")) (Math|Conversions|ToFloat(Integer) (.SnapValue (Utilities|Struct|BreakS_BuilderBlocks (stale _returnvalue))))) "0,0,0.010000"))
              (Variables|/Script/PluTool.BuilderBlock|SetmPlayerForward (Variables|Default|GetmVisibleBlock) (Math|Vector|GetForwardVector (Variables|/Game/FirstPerson/Blueprints/BP_FirstPersonCharacter.BP_FirstPersonCharacter_C|GetFirstPersonCamera _asbp_first_person_character)))
              (bind _output_get (Variables|Default|SetworldPos (Transformation|GetWorldLocation (Variables|/Script/PluTool.BuilderBlock|GetmMesh (Variables|Default|GetmVisibleBlock)))))
              (bind _output_get_2 (Variables|Default|SetworldRot (Transformation|GetWorldRotation (Variables|/Script/PluTool.BuilderBlock|GetmMesh (Variables|Default|GetmVisibleBlock)))))
              (if (Variables|/Script/PluTool.BuilderBlock|GetmPlaced (Variables|Default|GetmVisibleBlock))
                (Utilities|Array|Add (Variables|Default|GetBlocksInScene) (Variables|Default|GetmVisibleBlock))
                (Transformation|SetWorldLocationAndRotation (Variables|/Script/PluTool.BuilderBlock|GetmMesh (Variables|Default|GetmVisibleBlock)) _output_get _output_get_2 false false)
                (Rendering|Material|SetMaterial (Variables|/Script/PluTool.BuilderBlock|GetmMesh (Variables|Default|GetmVisibleBlock)) 0 "/Game/FPWeapon/Materials/BaseMaterial.BaseMaterial")
                (Variables|Default|SetmVisibleBlock 0)
                (Variables|Default|SetprevIndex -1)))))
        (else
          (if (Utilities|IsValid (Variables|Default|GetmVisibleBlock))
            (if (Variables|/Script/PluTool.BuilderBlock|GetmPlaced (Variables|Default|GetmVisibleBlock))
              _
              (else
                (Actor|DestroyActor (Variables|Default|GetmVisibleBlock)))))
          (bind _returnvalue (Utilities|GetDataTableRow "/Game/PluToolAssets/BBDataTables/DT_BBList.DT_BBList" (Utilities|String|StringToName (Utilities|String|ToString(Integer) (Variables|/Game/FirstPerson/Blueprints/BP_FirstPersonCharacter.BP_FirstPersonCharacter_C|GetBlockIndex _asbp_first_person_character))))
            (:then
              (Variables|Default|SetprevIndex (Variables|/Game/FirstPerson/Blueprints/BP_FirstPersonCharacter.BP_FirstPersonCharacter_C|GetBlockIndex _asbp_first_person_character))
              ;[0.0625 0.0625 0.0625] Spawn indexed actor as child of player and change material to green
              (bind _returnvalue_2 (Game|SpawnActorfromClass (.BlockObject (Utilities|Struct|BreakS_BuilderBlocks _returnvalue)) (Math|Transform|MakeTransform (+ (Class|KismetMathLibrary|VectorSnappedtoGrid (+ (Transformation|GetActorLocation _asbp_first_person_character) (* (Math|Vector|GetForwardVector (Variables|/Game/FirstPerson/Blueprints/BP_FirstPersonCharacter.BP_FirstPersonCharacter_C|GetFirstPersonCamera _asbp_first_person_character)) "750.000000,750.000000,750.000000")) (Math|Conversions|ToFloat(Integer) (.SnapValue (Utilities|Struct|BreakS_BuilderBlocks _returnvalue)))) "0,0,0.010000")) "Undefined" 0 0))
              (bind _output_get_3 (Variables|Default|SetmVisibleBlock _returnvalue_2))
              (bind _returnvalue_3 (Class|BuilderBlock|CheckforPrerequisites _returnvalue_2 (.Prerequisites (Utilities|Struct|BreakS_BuilderBlocks _returnvalue)) (Variables|Default|GetBlocksInScene)))
              (if _returnvalue_3
                (Variables|/Script/PluTool.BuilderBlock|SetmMeetsPrerequisites _output_get_3 true)
                (Rendering|Material|SetMaterial (Variables|/Script/PluTool.BuilderBlock|GetmMesh _returnvalue_2) 0 "/Game/PluToolAssets/Assets/Materials/M_BlueTrans.M_BlueTrans")
                (else
                  (Rendering|Material|SetMaterial (Variables|/Script/PluTool.BuilderBlock|GetmMesh _returnvalue_2) 0 "/Game/PluToolAssets/Assets/Materials/M_RedTrans.M_RedTrans")))))))
      (else
        ;[0.1406 0.1406 0.1406] Remove Visible block if it exists but we're not in Builder Mode
        (if (Utilities|IsValid (Variables|Default|GetmVisibleBlock)) :!label _label
          (Actor|DestroyActor (Variables|Default|GetmVisibleBlock))
          (Variables|Default|SetmVisibleBlock 0)
          (Variables|Default|SetprevIndex -1))))
    (else
      (goto _label))))

(fn ConstructionScript)