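; BP_BBWindowedWall is a windowed wall building block that tracks whether its placement prerequisites are met.
; On each begin overlap, it sets MMeetsPrerequisites true only if it overlaps at least two BP_BBCornerPiece actors and no StaticMeshActor.
; Any end overlap clears the flag without rechecking the remaining overlaps.
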(event EventBeginPlay)

(event EventTick
  (params (DeltaSeconds :type Float%20%28single-precision%29)))

(event Collision|EventActorBeginOverlap
  (params (OtherActor :type Actor%20Object%20Reference))
  ;[0.1 0.1 0.1] Making sure the Wall is colliding with 2 corner pieces
  (if (>= (Utilities|Array|Length (Collision|GetOverlappingActors "/Game/PluToolAssets/Blueprints/Builder/BuildingBlocks/BP_BBCornerPiece.BP_BBCornerPiece_C" :!class /Script/Engine.Actor)) 2)
    (if (> (Utilities|Array|Length (Collision|GetOverlappingActors "/Script/Engine.StaticMeshActor" :!class /Script/Engine.Actor)) 0)
      (Variables|Default|SetmMeetsPrerequisites false)
      (else
        (Variables|Default|SetmMeetsPrerequisites true)))
    (else
      (Variables|Default|SetmMeetsPrerequisites false))))

(event Collision|EventActorEndOverlap
  (params (OtherActor :type Actor%20Object%20Reference))
  ;[0.1 0.1 0.1] Making sure the Wall is colliding with 2 corner pieces
  (Variables|Default|SetmMeetsPrerequisites false))

(fn ConstructionScript)