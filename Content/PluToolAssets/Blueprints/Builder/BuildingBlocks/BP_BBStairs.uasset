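; Stairs building block for a builder tool that snaps to floor pieces and tracks whether its placement is valid.
; While unplaced, overlapping a BP_BBFloor moves it to the nearest of four points offset from that floor's bounds origin.
; Placement prerequisites pass only when it overlaps a floor and no static mesh actors.
; Ending an overlap while snapped clears both snapping and validity, and the first Tick initializes validity to false.
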(event EventBeginPlay)

(event EventTick
  (params (DeltaSeconds :type Float%20%28single-precision%29))
  (Utilities|FlowControl|DoOnce false
    (:Completed
      (Variables|Default|SetmMeetsPrerequisites false))))

(event Collision|EventActorBeginOverlap
  (params (OtherActor :type Actor%20Object%20Reference))
  (bind _origin (Collision|GetActorBounds OtherActor false true))
  (if (not (Variables|Default|GetmPlaced))
    (bind _asbp_bbfloor (Utilities|Casting|CastToBP_BBFloor OtherActor))
    (if (== OtherActor _asbp_bbfloor)
      (bind _output_get (Variables|Default|SetBounds (Utilities|Array|MakeArray (+ _origin "0.000000,250.000000,0.000000") (+ _origin "0.000000,-250.000000,0.000000") (+ _origin "-250.000000,0.000000,0.000000") (+ _origin "250.000000,0.000000,0.000000"))))
      (bind _output_get_2 (Variables|Default|SetclosestDistance 1e+04))
      (Variables|Default|Setdist _output_get_2)
      (for _array_element _output_get
        (bind _output_get_3 (Variables|Default|Setdist (Math|Float|Min(Float) (Math|Vector|Distance(Vector) _array_element (Transformation|GetActorLocation)) (Variables|Default|Getdist))))
        (if (< _output_get_3 (Variables|Default|GetclosestDistance))
          (Variables|Default|SetclosestDistance (Variables|Default|Getdist))
          (Variables|Default|Setlocation _array_element)))
      (Variables|Default|SetmSnapping true)
      (Transformation|SetActorLocation (Variables|Default|Getlocation) false false)
      ;[0.1 0.1 0.1] Making sure the Corner Piece is colliding with a floor
      (if (>= (Utilities|Array|Length (Collision|GetOverlappingActors "/Game/PluToolAssets/Blueprints/Builder/BuildingBlocks/BP_BBFloor.BP_BBFloor_C" :!class /Script/Engine.Actor)) 1)
        (if (> (Utilities|Array|Length (Collision|GetOverlappingActors "/Script/Engine.StaticMeshActor" :!class /Script/Engine.Actor)) 0)
          (Variables|Default|SetmMeetsPrerequisites false)
          (else
            (Variables|Default|SetmMeetsPrerequisites true)))
        (else
          (Variables|Default|SetmMeetsPrerequisites false))))))

(event Collision|EventActorEndOverlap
  (params (OtherActor :type Actor%20Object%20Reference))
  (if (Variables|Default|GetmSnapping)
    (Variables|Default|SetmSnapping false)
    (Variables|Default|SetmMeetsPrerequisites false)))

(fn ConstructionScript)